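; Base pawn for a powered tile-rotation circuit puzzle panel that the player possesses on use and leaves on exit.
; Short clicks rotate child-actor tiles, while holding and dragging rotates the view around the panel.
; Pathing spreads power from start tiles through connections by growing the list it iterates.
; With all end tiles powered, powered win-condition tiles complete it and fire a delayed mechanism trigger; otherwise it rotates end connections and flags errors.
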(event `TurnPowerOn`
  ;[1 1 1] Turn Power ON/OFF
  (if (not (`self.HasPower`))
    (set `self.HasPower` true)))

(event `self.ReceiveBeginPlay`
  ;[1 1 1] Init
  (`KismetSystemLibrary.Delay` 0.2)
  (`self.InitChain`)
  (add `/Game/Dynamic/Mechanisms/MechanismActionComponent.OnMechanismActionActivate` (`self.MechanismActionComponent`) (`|CreateDelegate` :!event `TurnPowerOn`))
  (add `/Game/Dynamic/Mechanisms/MechanismActionComponent.OnMechanismActionDeactivate` (`self.MechanismActionComponent`) (`|CreateDelegate` :!event `TurnPowerOff`)))

(event `/Game/Dynamic/Character/I_UseSystem.SetPower`
  (params (PowerUp :type Boolean))
  ;[1 1 1] Init
  (set `self.HasPower` PowerUp))

(event `TurnPowerOff`
  ;[1 1 1] Turn Power ON/OFF
  (if (`self.HasPower`)
    (set `self.HasPower` false)))

(event `/Game/Dynamic/Character/I_UseSystem.UseSelectedObject`
  (params (User :type "Pawn Object Reference"))
  ;[1 1 1] Taking and Losing Control of the puzzle panel
  (if (`self.HasPower`)
    (bind _output_get (set `self.User` User))
    (bind _output_get_2 (set `self.MyController` (`self.GetController` _output_get)))
    (message `/Game/Dynamic/Character/I_PawnMangement.ChangePawn` _output_get_2 self)
    (bind _playercontroller (message `/Game/Dynamic/Character/I_PawnMangement.GetPlayerControllerRef` _output_get_2))
    (`WidgetBlueprintLibrary.SetInputMode_GameAndUIEx` _playercontroller null)
    (set `PlayerController.bShowMouseCursor` true _playercontroller)
    (`self.StartedControllerSwapToPuzzle` _playercontroller)))

(event `ResetRotation`
  ;[1 1 1] Taking and Losing Control of the puzzle panel
  (set `self.CanInput` false)
  (set `self.CurrentRotation` (`SceneComponent.K2_GetComponentRotation` (`self.PuzzleCentraLeft/Right`)) :!label _label)
  (bind (_direction _alpha) (`Timeline|ResetRotationTimer` :!via `PlayFromStart`)
    (:`Update`
      (`SceneComponent.K2_SetWorldRotation` (`self.PuzzleCentraLeft/Right`) (`KismetMathLibrary.RLerp` (`self.CurrentRotation`) (`self.StartingRotation`) _alpha) false false))
    (:`Finished`
      (`self.ResetExit`)
      (set `self.CanInput` true))))

(event `/Game/Dynamic/Character/I_InputControls.ExitPressed`
  (bind _returnvalue (`self.GetController`))
  ;[1 1 1] Taking and Losing Control of the puzzle panel
  (`/Engine/EditorBlueprintResources/StandardMacros.DoOnce` false :!label _label_2
    (:`Completed`
      (`self.StartedControllerSwapToCharacter` _returnvalue)
      (bind _output_get (set `self.MyController` _returnvalue))
      (message `/Game/Dynamic/Character/I_PawnMangement.ChangePawn` _output_get (`self.User`))
      (bind _playercontroller (message `/Game/Dynamic/Character/I_PawnMangement.GetPlayerControllerRef` _output_get))
      (`WidgetBlueprintLibrary.SetInputMode_GameOnly` _playercontroller)
      (set `PlayerController.bShowMouseCursor` false _playercontroller)
      (set `self.User` null)
      (set `self.MyController` null)
      (goto _label))))

(event `ResetExit`
  ;[1 1 1] Taking and Losing Control of the puzzle panel
  (goto _label_2 :!via `Reset`))

(event `/Game/Dynamic/Character/I_InputControls.UsePressed`
  ;[1 1 1] Left Mouse Button Input
  (bind _returnvalue (`KismetSystemLibrary.K2_SetTimerDelegate` (delegate `MouseDown`) 0.2))
  (set `self.MouseButtonDownTimerHandle` _returnvalue))

(event `/Game/Dynamic/Character/I_InputControls.MiddleMousePressed`
  ;[1 1 1] Middle Mouse Input
  (`self.ResetRotation`)
  (`self.ResetCameraPressed`))

(event `MouseDown`
  ;[1 1 1] Left Mouse Button Input
  (set `self.MouseButtonIsDown` true))

(event `/Game/Dynamic/Character/I_InputControls.ResetPressed`
  ;[1 1 1] Reset All Tiles
  (if (`self.IsCompleted`)
    _
    (elif (`self.CanInput`)
      (for _array_element (`self.Tiles`)
        (message `/Game/Dynamic/PuzzlePanel/Tiles/I_Tile.ResetTile` _array_element)))))

(event `/Game/Dynamic/Character/I_InputControls.UseReleased`
  ;[1 1 1] Left Mouse Button Input
  (`KismetSystemLibrary.K2_ClearAndInvalidateTimerHandle` (`self.MouseButtonDownTimerHandle`))
  (if (`self.MouseButtonIsDown`)
    (set `self.MouseButtonIsDown` false)
    (else
      (`self.HitDetection`))))

(event `HitDetection`
  ;[1 1 1] Left Mouse Button Input
  (if (`self.IsCompleted`)
    _
    (elif (`self.CanInput`)
      (bind _output_get (set `self.MyController` (`self.GetController`)))
      (bind _playercontroller (message `/Game/Dynamic/Character/I_PawnMangement.GetPlayerControllerRef` _output_get))
      (bind (_hitresult _returnvalue) (`PlayerController.GetHitResultUnderCursorByChannel` _playercontroller "TraceTypeQuery3" true))
      (if _returnvalue
        (bind _tileref (message `/Game/Dynamic/PuzzlePanel/Tiles/I_Tile.GetSpinableTileRef` (`.HitActor` (`GameplayStatics.BreakHitResult` _hitresult))))
        (`/Engine/EditorBlueprintResources/StandardMacros.IsValid` _tileref
          (:`Is Valid`
            (if (`KismetArrayLibrary.Array_Contains` (`self.Tiles`) _tileref)
              (message `/Game/Dynamic/PuzzlePanel/Tiles/I_Tile.RotateTile` _tileref))))))))

(event `/Game/Dynamic/Character/I_InputControls.Turn`
  (params (Scale :type "Float (single-precision)"))
  ;[1 1 1] Mouse Movement Input
  (if (`self.MouseButtonIsDown`)
    (`SceneComponent.K2_AddWorldRotation` (`self.PuzzleCentraLeft/Right`) (`KismetMathLibrary.MakeRotator` 0.0 0.0 (* (* -1 Scale) (`self.RotationRate`))) false false)))

(event `/Game/Dynamic/Character/I_InputControls.LookUp/Down`
  (params (Scale :type "Float (single-precision)"))
  ;[1 1 1] Mouse Movement Input
  (if (`self.MouseButtonIsDown`)
    (`SceneComponent.K2_AddLocalRotation` (`self.PuzzleCentraUp/Down`) (`KismetMathLibrary.MakeRotator` 0.0 (* Scale (`self.RotationRate`))) false false)))

(fn `AddTileToCorrectList`
  (params (ChildActor :type "Actor Object Reference"))
  (bind _tileref (message `/Game/Dynamic/PuzzlePanel/Tiles/I_Tile.GetSpinableTileRef` ChildActor))
  (`/Engine/EditorBlueprintResources/StandardMacros.IsValid` _tileref
    (:`Is Valid`
      (`KismetArrayLibrary.Array_AddUnique` (`self.Tiles`) _tileref)
      (add `/Game/Dynamic/PuzzlePanel/Tiles/BP_SpinableTile.OnFinishRotating` _tileref (`|CreateDelegate` :!event `CalculatePathing`)))
    (:`Is Not Valid`
      (bind _starttileref (message `/Game/Dynamic/PuzzlePanel/Tiles/I_Tile.GetStartTileRef` ChildActor))
      (`/Engine/EditorBlueprintResources/StandardMacros.IsValid` _starttileref
        (:`Is Valid`
          (`KismetArrayLibrary.Array_AddUnique` (`self.StartTiles`) _starttileref))
        (:`Is Not Valid`
          (bind _endtileref (message `/Game/Dynamic/PuzzlePanel/Tiles/I_Tile.GetEndTileRef` ChildActor))
          (`/Engine/EditorBlueprintResources/StandardMacros.IsValid` _endtileref
            (:`Is Valid`
              (`KismetArrayLibrary.Array_AddUnique` (`self.EndTiles`) _endtileref))))))))

(fn `CalculatePathing`
  (locals (ConnectTiles :type "Array of Actor Object Reference"))
  (for _array_element (`self.StartTiles`)
    (`KismetArrayLibrary.Array_AddUnique` (`local.ConnectTiles`) _array_element))
  (for _array_element_2 (`local.ConnectTiles`)
    (bind _connections (message `/Game/Dynamic/PuzzlePanel/Tiles/I_Tile.GetAllConnections` _array_element_2))
    (for _array_element_3 _connections
      (`KismetArrayLibrary.Array_AddUnique` (`local.ConnectTiles`) _array_element_3)))
  (for _array_element_4 (`self.Tiles`)
    (if (not (`KismetArrayLibrary.Array_Contains` (`local.ConnectTiles`) _array_element_4))
      (message `/Game/Dynamic/PuzzlePanel/Tiles/I_Tile.PowerDown` _array_element_4)))
  (for _array_element_5 (`self.EndTiles`)
    (if (not (`KismetArrayLibrary.Array_Contains` (`local.ConnectTiles`) _array_element_5))
      (message `/Game/Dynamic/PuzzlePanel/Tiles/I_Tile.PowerDown` _array_element_5)))
  (message `/Game/Dynamic/PuzzlePanel/Tiles/I_Tile.PowerUp` (`local.ConnectTiles`))
  (`self.CheckWinCondition`))

(fn `CheckIfWinConditionTile`
  (params (BaseTileRef :type "/Game/Dynamic/PuzzlePanel/Tiles/BP_BaseTile Object Reference"))
  (bind _iswincondition (message `/Game/Dynamic/PuzzlePanel/Tiles/I_Tile.GetIsWinCondition` BaseTileRef))
  (if _iswincondition
    (`KismetArrayLibrary.Array_AddUnique` (`self.WinConditionTiles`) BaseTileRef))
  (return))

(fn `CheckWinCondition`
  (locals (HasFailed :type Boolean))
  (for _array_element (`self.EndTiles`)
    (bind _ispowered (message `/Game/Dynamic/PuzzlePanel/Tiles/I_Tile.GetIsPowered` _array_element))
    (if (not _ispowered)
      (set `local.HasFailed` true)))
  (if (not (`local.HasFailed`))
    (for _array_element_2 (`self.WinConditionTiles`)
      (bind _ispowered_2 (message `/Game/Dynamic/PuzzlePanel/Tiles/I_Tile.GetIsPowered` _array_element_2))
      (if (not _ispowered_2)
        (set `local.HasFailed` true)))
    (if (`local.HasFailed`)
      (`self.LosePuzzle`)
      (else
        (`self.WinPuzzle`)))))

(fn `DelayBeforeCompletion`
  (`/Game/Dynamic/Mechanisms/MechanismTriggerComponent.ActivateTrigger` (`self.MechanismTriggerComponent`)))

(fn `GetMechanismTriggerRef`
  (returns (TriggerRef :type "/Game/Dynamic/Mechanisms/MechanismTriggerComponent Object Reference"))
  (return (`self.MechanismTriggerComponent`)))

(fn `InitChain`
  (bind _puzzlecentraleft_right (`self.PuzzleCentraLeft/Right`))
  (`self.SetUpTilesToIgnore`)
  (set `self.StartingRotation` (`SceneComponent.K2_GetComponentRotation` _puzzlecentraleft_right))
  (for _array_element (`SceneComponent.GetChildrenComponents` _puzzlecentraleft_right true)
    (bind _aschild_actor_component (cast `ChildActorComponent` _array_element))
    (bind _childactor (`ChildActorComponent.ChildActor` _aschild_actor_component))
    (bind _basetileref (message `/Game/Dynamic/PuzzlePanel/Tiles/I_Tile.GetBaseTileRef` _childactor))
    (`self.CheckIfWinConditionTile` _basetileref)
    (`self.AddTileToCorrectList` _childactor)
    (message `/Game/Dynamic/PuzzlePanel/Tiles/I_Tile.InitTile` _childactor))
  (`self.CalculatePathing`))

(fn `LosePuzzle`
  (for _array_element (`self.EndTiles`)
    (bind _connections (message `/Game/Dynamic/PuzzlePanel/Tiles/I_Tile.GetAllConnections` _array_element))
    (for _array_element_2 _connections
      (message `/Game/Dynamic/PuzzlePanel/Tiles/I_Tile.RotateTile` _array_element_2)))
  (`GameplayStatics.PlaySoundAtLocation` (`self.FailSound`) (`self.K2_GetActorLocation`) (struct) 1.0 1.0 0.0 null null null)
  (for _array_element_3 (`self.WinConditionTiles`)
    (bind _ispowered (message `/Game/Dynamic/PuzzlePanel/Tiles/I_Tile.GetIsPowered` _array_element_3))
    (if (not _ispowered)
      (message `/Game/Dynamic/PuzzlePanel/Tiles/I_Tile.EnableErrorOnTile` _array_element_3))))

(fn `ResetCameraPressed`
  (returns (Ignore :type Boolean))
  (return false))

(fn `SetUpTilesToIgnore`)

(fn `StartedControllerSwapToCharacter`
  (params (Controller :type "Controller Object Reference"))
  (returns (Ignore :type Boolean))
  (return false))

(fn `StartedControllerSwapToPuzzle`
  (params (Controller :type "Controller Object Reference"))
  (returns (Ignore :type Boolean))
  (return false))

(fn `UserConstructionScript`)

(fn `WinPuzzle`
  (set `self.IsCompleted` true)
  (set `self.CanInput` false)
  (`GameplayStatics.PlaySoundAtLocation` (`self.SucessSound`) (`self.K2_GetActorLocation`) (struct) 1.0 1.0 0.0 null null null)
  (`KismetSystemLibrary.K2_SetTimerDelegate` (`|CreateDelegate` :!event `DelayBeforeCompletion`) (`self.CompletionDelay`))
  (return))