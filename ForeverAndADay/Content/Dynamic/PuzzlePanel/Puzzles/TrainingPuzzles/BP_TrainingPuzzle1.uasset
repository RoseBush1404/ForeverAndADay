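; BP_TrainingPuzzle1 is a tutorial puzzle panel that teaches possessing the puzzle, rotating a tile and leaving it.
; A detection sphere triggers the left-mouse hint until possession, and winning triggers the right-mouse hint until the player returns to the character.
; On possession it shows a runtime-added pulsing flipbook circle on the straight tile plus a left-mouse hint.
; One-shot flags and controller-swap overrides retire each prompt.
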(event `self.ReceiveBeginPlay`
  ;[1 1 1] Teaching Rotation
  (`KismetSystemLibrary.Delay` 0.2)
  (`self.InitChain`)
  (bind _tileref (message `/Game/Dynamic/PuzzlePanel/Tiles/I_Tile.GetSpinableTileRef` (`ChildActorComponent.ChildActor` (`self.StrightTile`))))
  (`/Engine/EditorBlueprintResources/StandardMacros.IsValid` _tileref
    (:`Is Valid`
      (add `/Game/Dynamic/PuzzlePanel/Tiles/BP_SpinableTile.OnFinishRotating` _tileref (`|CreateDelegate` :!event `TeachingTileRotation`))
      (bind _returnvalue (`AddComponent|NODE_AddPaperFlipbookComponent-0` :`self` _tileref :`RelativeTransform` (`KismetMathLibrary.MakeTransform` (0.0 0.0 1.0) (struct :`Roll` -90.0) (0.01 0.01 0.01))))
      (set `self.CircleFlipBook` _returnvalue)
      (`PaperFlipbookComponent.SetFlipbook` _returnvalue "/Game/Static/UI/PusleCircle/FB_PulseCircle.FB_PulseCircle")
      (`PaperFlipbookComponent.SetSpriteColor` :`self` _returnvalue))))

(event `self.ReceivePossessed`
  (params (NewController :type "Controller Object Reference"))
  ;[1 1 1] Teaching Rotation
  (if (not (`self.TeachedRotation`))
    (`self.FadeInCircle`)
    (`KismetSystemLibrary.Delay` 0.25)
    (message `/Game/Dynamic/UI/I_ControlWidgetFade.FadeInLeftMouse` (`self.GetController`))))

(event `TeachingTileRotation`
  ;[1 1 1] Teaching Rotation
  (if (not (`self.TeachedRotation`))
    (`self.FadeOutCircle`)
    (set `self.TeachedRotation` true)
    (message `/Game/Dynamic/UI/I_ControlWidgetFade.FadeOutLeftMouse` (`self.GetController`))))

(event `FadeInCircle`
  (bind _circleflipbook (`self.CircleFlipBook`))
  ;[1 1 1] Teaching Rotation
  (`/Engine/EditorBlueprintResources/StandardMacros.IsValid` _circleflipbook
    (:`Is Valid`
      (`PaperFlipbookComponent.SetSpriteColor` _circleflipbook (make `LinearColor` 1.0 1.0 1.0 1.0)))))

(event `FadeOutCircle`
  (bind _circleflipbook (`self.CircleFlipBook`))
  ;[1 1 1] Teaching Rotation
  (`/Engine/EditorBlueprintResources/StandardMacros.IsValid` _circleflipbook
    (:`Is Valid`
      (`PaperFlipbookComponent.SetSpriteColor` _circleflipbook (make `LinearColor` 1.0 1.0 1.0)))))

(event `self.PlayerDectionSphere.OnComponentBeginOverlap`
  (params (OverlappedComponent :type "PrimitiveComponent Object Reference") (OtherActor :type "Actor Object Reference") (OtherComp :type "PrimitiveComponent Object Reference") (OtherBodyIndex :type Integer) (bFromSweep :type Boolean) (SweepResult :type "HitResult Structure (by ref)"))
  (bind _returnvalue (`GameplayStatics.GetPlayerPawn` 0))
  ;[1 1 1] Teaching Posses
  (if (`self.TeachedPosses`)
    _
    (elif (== OtherActor _returnvalue)
      (message `/Game/Dynamic/UI/I_ControlWidgetFade.FadeInLeftMouse` (`self.GetController` _returnvalue)))))

(event `self.PlayerDectionSphere.OnComponentEndOverlap`
  (params (OverlappedComponent :type "PrimitiveComponent Object Reference") (OtherActor :type "Actor Object Reference") (OtherComp :type "PrimitiveComponent Object Reference") (OtherBodyIndex :type Integer))
  (bind _returnvalue (`GameplayStatics.GetPlayerPawn` 0))
  ;[1 1 1] Teaching Posses
  (if (`self.TeachedPosses`)
    _
    (elif (== OtherActor _returnvalue)
      (message `/Game/Dynamic/UI/I_ControlWidgetFade.FadeOutLeftMouse` (`self.GetController` _returnvalue)))))

(fn `StartedControllerSwapToCharacter`
  (params (Controller :type "Controller Object Reference"))
  (returns (Ignore :type Boolean))
  (if (not (`self.TeachedUnposses`))
    (set `self.TeachedUnposses` true)
    (message `/Game/Dynamic/UI/I_ControlWidgetFade.FadeOutRightMouse` Controller))
  (if (`self.TeachedRotation`)
    (return false)
    (else
      (message `/Game/Dynamic/UI/I_ControlWidgetFade.FadeOutLeftMouse` Controller))))

(fn `StartedControllerSwapToPuzzle`
  (params (Controller :type "Controller Object Reference"))
  (returns (Ignore :type Boolean))
  (if (`self.TeachedPosses`)
    (return false)
    (else
      (message `/Game/Dynamic/UI/I_ControlWidgetFade.FadeOutLeftMouse` Controller)
      (set `self.TeachedPosses` true)
      (return false))))

(fn `UserConstructionScript`
  (`parent.UserConstructionScript`))

(fn `WinPuzzle`
  (`parent.WinPuzzle`)
  (if (not (`self.TeachedUnposses`))
    (message `/Game/Dynamic/UI/I_ControlWidgetFade.FadeInRightMouse` (`self.GetController`))
    (return)))