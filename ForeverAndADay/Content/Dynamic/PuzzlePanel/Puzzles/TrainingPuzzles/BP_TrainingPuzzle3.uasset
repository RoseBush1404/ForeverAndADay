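; BP_TrainingPuzzle3 is a training puzzle that teaches camera rotation, then camera reset, through on-screen mouse prompts.
; On possession it shows drag and left-mouse hints, while a looping timer polls for a held mouse button as proof of rotation.
; That swaps the hints for a middle-mouse prompt, which pressing reset dismisses.
; Swapping back to the character clears prompts and timer, restarting the lesson if reset was shown but never used.
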(event `self.ReceivePossessed`
  (params (NewController :type "Controller Object Reference"))
  (`KismetSystemLibrary.Delay` 0.25)
  (if (not (`self.TeachedRotateCamera`))
    (message `/Game/Dynamic/UI/I_ControlWidgetFade.FadeInDragLine` NewController)
    (message `/Game/Dynamic/UI/I_ControlWidgetFade.StartDragAnimation` NewController)
    (message `/Game/Dynamic/UI/I_ControlWidgetFade.FadeInLeftMouse` NewController))
  (if (not (`self.TeachedShowResetCamera`))
    (bind _returnvalue (`KismetSystemLibrary.K2_SetTimerDelegate` (`|CreateDelegate` :!event `CheckToSeeIfCameraHasRotated`) 0.1 true))
    (set `self.CheckHandle` _returnvalue)))

(event `CheckToSeeIfCameraHasRotated`
  (bind _returnvalue (`self.GetController`))
  (if (`self.TeachedShowResetCamera`)
    _
    (elif (`self.MouseButtonIsDown`)
      (set `self.TeachedShowResetCamera` true)
      (set `self.TeachedRotateCamera` true)
      (message `/Game/Dynamic/UI/I_ControlWidgetFade.FadeOutDragLine` _returnvalue)
      (message `/Game/Dynamic/UI/I_ControlWidgetFade.FadeOutLeftMouse` _returnvalue)
      (message `/Game/Dynamic/UI/I_ControlWidgetFade.FadeInMiddleMouse` _returnvalue)
      (`KismetSystemLibrary.K2_ClearAndInvalidateTimerHandle` (`self.CheckHandle`))
      (`self.StopDragAnimationAfterDelay` _returnvalue))))

(event `StopDragAnimationAfterDelay`
  (params (Target :type "Controller Object Reference"))
  (`KismetSystemLibrary.Delay` 0.5)
  (message `/Game/Dynamic/UI/I_ControlWidgetFade.StopDragAnimation` Target))

(fn `ResetCameraPressed`
  (returns (Ignore :type Boolean))
  (if (`self.TeachedHideResetCamera`)
    (return false)
    (else
      (message `/Game/Dynamic/UI/I_ControlWidgetFade.FadeOutMiddleMouse` (`self.GetController`))
      (set `self.TeachedHideResetCamera` true)
      (return false))))

(fn `StartedControllerSwapToCharacter`
  (params (Controller :type "Controller Object Reference"))
  (returns (Ignore :type Boolean))
  (if (not (`self.TeachedRotateCamera`))
    (message `/Game/Dynamic/UI/I_ControlWidgetFade.FadeOutDragLine` Controller)
    (message `/Game/Dynamic/UI/I_ControlWidgetFade.FadeOutLeftMouse` Controller)
    (`self.StopDragAnimationAfterDelay` Controller))
  (`KismetSystemLibrary.K2_ClearAndInvalidateTimerHandle` (`self.CheckHandle`))
  (if (`self.TeachedShowResetCamera`)
    (if (`self.TeachedHideResetCamera`)
      (return false)
      (else
        (message `/Game/Dynamic/UI/I_ControlWidgetFade.FadeOutMiddleMouse` Controller)
        (set `self.TeachedShowResetCamera` false)
        (set `self.TeachedHideResetCamera` false)
        (set `self.TeachedRotateCamera` false)
        (return false)))
    (else
      (return false))))

(fn `UserConstructionScript`
  (`parent.UserConstructionScript`))