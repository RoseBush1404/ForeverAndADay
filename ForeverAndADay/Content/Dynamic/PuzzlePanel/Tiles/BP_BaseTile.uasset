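; Base puzzle-panel tile that tracks its connected tiles and can be powered up or down, swapping its mesh material to show the state.
; Connections are added or removed from other actors' tile references, and getters expose them along with power and win-condition flags.
; Type getters return self for base tile and empty for start, end and spinnable tiles.
; InitCollider moves a collider to zero and back, apparently to refresh overlaps.
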(fn `AddConnection`
  (params (`Other Actor` :type "Actor Object Reference"))
  (bind _actorref (message `/Game/Dynamic/PuzzlePanel/Tiles/I_Tile.GetTileActorRef` `Other Actor`))
  (`/Engine/EditorBlueprintResources/StandardMacros.IsValid` _actorref
    (:`Is Valid`
      (`KismetArrayLibrary.Array_AddUnique` (`self.Connections`) _actorref))))

(fn `GetAllConnections`
  (returns (Connections :type "Array of Actor Object Reference"))
  (return (`self.Connections`)))

(fn `GetBaseTileRef`
  (returns (BaseTileRef :type "/Game/Dynamic/PuzzlePanel/Tiles/BP_BaseTile Object Reference"))
  (return self))

(fn `GetEndTileRef`
  (returns (EndTileRef :type "/Game/Dynamic/PuzzlePanel/Tiles/BP_BaseEndTile Object Reference"))
  (return null))

(fn `GetIsPowered`
  (returns (IsPowered :type Boolean))
  (return (`self.IsPowered`)))

(fn `GetIsWinCondition`
  (returns (IsWinCondition :type Boolean))
  (return (`self.IsWinCondition`)))

(fn `GetSpinableTileRef`
  (returns (TileRef :type "/Game/Dynamic/PuzzlePanel/Tiles/BP_SpinableTile Object Reference"))
  (return null))

(fn `GetStartTileRef`
  (returns (StartTileRef :type "/Game/Dynamic/PuzzlePanel/Tiles/BP_BaseStartTile Object Reference"))
  (return null))

(fn `GetTileActorRef`
  (returns (ActorRef :type "Actor Object Reference"))
  (return self))

(fn `InitCollider`
  (params (Collider :type "SphereComponent Object Reference"))
  (locals (StoredLocation :type "Vector Structure"))
  (bind _output_get (set `local.StoredLocation` (`SceneComponent.RelativeLocation` Collider)))
  (`SceneComponent.K2_SetRelativeLocation` Collider (0.0 0.0 0.0) false false)
  (`SceneComponent.K2_SetRelativeLocation` Collider _output_get false false))

(fn `PowerDown`
  (returns (Success :type Boolean))
  (`PrimitiveComponent.SetMaterial` (`self.StaticMesh`) 0 (`self.PowerDownMaterial`))
  (set `self.IsPowered` false)
  (return true))

(fn `PowerUp`
  (returns (Success :type Boolean))
  (`PrimitiveComponent.SetMaterial` (`self.StaticMesh`) 0 (`self.PowerUpMaterial`))
  (set `self.IsPowered` true)
  (return true))

(fn `RemoveConnection`
  (params (OtherActor :type "Actor Object Reference"))
  (bind _actorref (message `/Game/Dynamic/PuzzlePanel/Tiles/I_Tile.GetTileActorRef` OtherActor))
  (`/Engine/EditorBlueprintResources/StandardMacros.IsValid` _actorref
    (:`Is Valid`
      (`KismetArrayLibrary.Array_RemoveItem` (`self.Connections`) _actorref))))

(fn `UserConstructionScript`)