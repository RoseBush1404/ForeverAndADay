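; BP_BaseStartTile is the start tile of a tile-based puzzle panel, with a single connection point on its east side.
; InitTile initializes the east collider, whose overlap begin and end events add and remove connections to other actors.
; GetStartTileRef returns the tile itself, and PowerUp and PowerDown both simply return true without changing any state.
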(event `self.EastCollider.OnComponentBeginOverlap`
  (params (OverlappedComponent :type "PrimitiveComponent Object Reference") (OtherActor :type "Actor Object Reference") (OtherComp :type "PrimitiveComponent Object Reference") (OtherBodyIndex :type Integer) (bFromSweep :type Boolean) (SweepResult :type "HitResult Structure (by ref)"))
  ;[1 1 1] Connection Adding/Removing
  (`self.AddConnection` OtherActor))

(event `self.EastCollider.OnComponentEndOverlap`
  (params (OverlappedComponent :type "PrimitiveComponent Object Reference") (OtherActor :type "Actor Object Reference") (OtherComp :type "PrimitiveComponent Object Reference") (OtherBodyIndex :type Integer))
  ;[1 1 1] Connection Adding/Removing
  (`self.RemoveConnection` OtherActor))

(event `/Game/Dynamic/PuzzlePanel/Tiles/I_Tile.InitTile`
  ;[1 1 1] Init Tile
  (`self.InitCollider` (`self.EastCollider`)))

(fn `GetStartTileRef`
  (returns (StartTileRef :type "/Game/Dynamic/PuzzlePanel/Tiles/BP_BaseStartTile Object Reference"))
  (return self))

(fn `PowerDown`
  (returns (Success :type Boolean))
  (return true))

(fn `PowerUp`
  (returns (Success :type Boolean))
  (return true))

(fn `UserConstructionScript`)