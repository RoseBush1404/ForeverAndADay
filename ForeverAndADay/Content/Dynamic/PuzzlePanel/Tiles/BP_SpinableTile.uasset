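; Spinnable puzzle-panel tile that rotates by a set yaw step and shows powered, unpowered or temporary error materials.
; Four directional colliders add and remove connections to overlapping actors.
; Timelines drive the lifted spin with sound and the reset to the rotation captured shortly after BeginPlay, locking re-entry and signalling on finish.
; The error material reverts on a timer, which PowerUp cancels, while PowerDown leaves an active error untouched.
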(event `self.NorthCollider.OnComponentBeginOverlap`
  (params (OverlappedComponent :type "PrimitiveComponent Object Reference") (OtherActor :type "Actor Object Reference") (OtherComp :type "PrimitiveComponent Object Reference") (OtherBodyIndex :type Integer) (bFromSweep :type Boolean) (SweepResult :type "HitResult Structure (by ref)"))
  ;[1 1 1] Collision Dection
  (`self.AddConnection` OtherActor))

(event `/Game/Dynamic/PuzzlePanel/Tiles/I_Tile.EnableErrorOnTile`
  (bind _errormaterial (`self.ErrorMaterial`))
  ;[1 1 1] Error Material Change
  (`/Engine/EditorBlueprintResources/StandardMacros.IsValid` _errormaterial
    (:`Is Valid`
      (`PrimitiveComponent.SetMaterial` (`self.StaticMesh`) 0 _errormaterial)
      (bind _returnvalue (`KismetSystemLibrary.K2_SetTimerDelegate` (delegate `ResetMaterial`) 1.5))
      (set `self.ErrorTimerHandle` _returnvalue))))

(event `/Game/Dynamic/PuzzlePanel/Tiles/I_Tile.RotateTile`
  (bind _defaultsceneroot (`self.DefaultSceneRoot`))
  ;[1 1 1] Rotate Tile
  (if (not (`self.IsRotating`))
    (set `self.IsRotating` true)
    (`self.StoreTileStartingRotationValues`)
    (bind (_direction _rotationalpha _locationalpha) (`Timeline|RotateTileTimeLine` :!via `PlayFromStart`)
      (:`Update`
        (`SceneComponent.K2_SetRelativeRotation` _defaultsceneroot (`self.LerpTileRotation` _rotationalpha) false false)
        (`SceneComponent.K2_SetRelativeLocation` _defaultsceneroot (`self.LerpTileLocation` _locationalpha) false false))
      (:`Finished`
        (set `self.IsRotating` false)
        (`self.OnFinishRotating`))
      (:`SoundTrigger`
        (`self.PlayRotationSFX`)))))

(event `self.NorthCollider.OnComponentEndOverlap`
  (params (OverlappedComponent :type "PrimitiveComponent Object Reference") (OtherActor :type "Actor Object Reference") (OtherComp :type "PrimitiveComponent Object Reference") (OtherBodyIndex :type Integer))
  ;[1 1 1] Collision Dection
  (`self.RemoveConnection` OtherActor))

(event `ResetMaterial`
  ;[1 1 1] Error Material Change
  (`PrimitiveComponent.SetMaterial` (`self.StaticMesh`) 0 (`self.PowerDownMaterial`)))

(event `self.SouthCollider.OnComponentBeginOverlap`
  (params (OverlappedComponent :type "PrimitiveComponent Object Reference") (OtherActor :type "Actor Object Reference") (OtherComp :type "PrimitiveComponent Object Reference") (OtherBodyIndex :type Integer) (bFromSweep :type Boolean) (SweepResult :type "HitResult Structure (by ref)"))
  ;[1 1 1] Collision Dection
  (`self.AddConnection` OtherActor))

(event `/Game/Dynamic/PuzzlePanel/Tiles/I_Tile.InitTile`
  ;[1 1 1] Init Tile
  (`self.InitCollider` (`self.EastCollider`))
  (`self.InitCollider` (`self.WestCollider`))
  (`self.InitCollider` (`self.NorthCollider`))
  (`self.InitCollider` (`self.SouthCollider`)))

(event `self.SouthCollider.OnComponentEndOverlap`
  (params (OverlappedComponent :type "PrimitiveComponent Object Reference") (OtherActor :type "Actor Object Reference") (OtherComp :type "PrimitiveComponent Object Reference") (OtherBodyIndex :type Integer))
  ;[1 1 1] Collision Dection
  (`self.RemoveConnection` OtherActor))

(event `self.ReceiveBeginPlay`
  ;[1 1 1] ResetTile
  (`KismetSystemLibrary.Delay` 0.2)
  (set `self.SpawnedRotation` (`SceneComponent.RelativeRotation` (`self.DefaultSceneRoot`))))

(event `self.WestCollider.OnComponentBeginOverlap`
  (params (OverlappedComponent :type "PrimitiveComponent Object Reference") (OtherActor :type "Actor Object Reference") (OtherComp :type "PrimitiveComponent Object Reference") (OtherBodyIndex :type Integer) (bFromSweep :type Boolean) (SweepResult :type "HitResult Structure (by ref)"))
  ;[1 1 1] Collision Dection
  (`self.AddConnection` OtherActor))

(event `/Game/Dynamic/PuzzlePanel/Tiles/I_Tile.ResetTile`
  (bind _defaultsceneroot (`self.DefaultSceneRoot`))
  ;[1 1 1] ResetTile
  (if (not (`self.IsRotating`))
    (set `self.IsRotating` true)
    (`self.StoreTileStartingRotationValues`)
    (bind (_direction _rotationalpha _locationalpha) (`Timeline|ResetTileTimeLine` :!via `PlayFromStart`)
      (:`Update`
        (`SceneComponent.K2_SetRelativeRotation` _defaultsceneroot (`KismetMathLibrary.RLerp` (`self.StartingRotation`) (`self.SpawnedRotation`) _rotationalpha) false false)
        (`SceneComponent.K2_SetRelativeLocation` _defaultsceneroot (`self.LerpTileLocation` _locationalpha) false false))
      (:`Finished`
        (set `self.IsRotating` false)
        (`self.OnFinishRotating`)))))

(event `self.WestCollider.OnComponentEndOverlap`
  (params (OverlappedComponent :type "PrimitiveComponent Object Reference") (OtherActor :type "Actor Object Reference") (OtherComp :type "PrimitiveComponent Object Reference") (OtherBodyIndex :type Integer))
  ;[1 1 1] Collision Dection
  (`self.RemoveConnection` OtherActor))

(event `self.EastCollider.OnComponentBeginOverlap`
  (params (OverlappedComponent :type "PrimitiveComponent Object Reference") (OtherActor :type "Actor Object Reference") (OtherComp :type "PrimitiveComponent Object Reference") (OtherBodyIndex :type Integer) (bFromSweep :type Boolean) (SweepResult :type "HitResult Structure (by ref)"))
  ;[1 1 1] Collision Dection
  (`self.AddConnection` OtherActor))

(event `self.EastCollider.OnComponentEndOverlap`
  (params (OverlappedComponent :type "PrimitiveComponent Object Reference") (OtherActor :type "Actor Object Reference") (OtherComp :type "PrimitiveComponent Object Reference") (OtherBodyIndex :type Integer))
  ;[1 1 1] Collision Dection
  (`self.RemoveConnection` OtherActor))

(fn `GetSpinableTileRef`
  (returns (TileRef :type "/Game/Dynamic/PuzzlePanel/Tiles/BP_SpinableTile Object Reference"))
  (return self))

(fn `LerpTileLocation`
  (params (Alpha :type "Float (double-precision)"))
  (returns (ReturnValue :type "Vector Structure"))
  (bind _startinglocation (`self.StartingLocation`))
  (return (`KismetMathLibrary.VLerp` _startinglocation (`KismetMathLibrary.MakeVector` (.x _startinglocation) (.y _startinglocation) (+ (.z _startinglocation) (`self.TileRotationHight`))) Alpha)))

(fn `LerpTileRotation`
  (params (Alpha :type "Float (double-precision)"))
  (returns (ReturnValue :type "Rotator Structure"))
  (bind _startingrotation (`self.StartingRotation`))
  (return (`KismetMathLibrary.RLerp` _startingrotation (`KismetMathLibrary.MakeRotator` (.roll _startingrotation) (.pitch _startingrotation) (+ (.yaw _startingrotation) (`self.TileRotationAmount`))) Alpha)))

(fn `PlayRotationSFX`
  (`GameplayStatics.PlaySoundAtLocation` (`self.RotationAudio`) (`self.K2_GetActorLocation`) (struct) 1.0 1.0 0.0 null null null))

(fn `PowerDown`
  (returns (Success :type Boolean))
  (bind _staticmesh (`self.StaticMesh`))
  (if (!= (`PrimitiveComponent.GetMaterial` _staticmesh 0) (`self.ErrorMaterial`))
    (`PrimitiveComponent.SetMaterial` _staticmesh 0 (`self.PowerDownMaterial`))
    (set `self.IsPowered` false))
  (return true))

(fn `PowerUp`
  (returns (Success :type Boolean))
  (bind _errortimerhandle (`self.ErrorTimerHandle`))
  (`PrimitiveComponent.SetMaterial` (`self.StaticMesh`) 0 (`self.PowerUpMaterial`))
  (set `self.IsPowered` true)
  (if (`KismetSystemLibrary.K2_IsTimerActiveHandle` _errortimerhandle)
    (`KismetSystemLibrary.K2_ClearAndInvalidateTimerHandle` _errortimerhandle))
  (return true))

(fn `StoreTileStartingRotationValues`
  (bind _defaultsceneroot (`self.DefaultSceneRoot`))
  (set `self.StartingRotation` (`SceneComponent.RelativeRotation` _defaultsceneroot))
  (set `self.StartingLocation` (`SceneComponent.RelativeLocation` _defaultsceneroot)))

(fn `UserConstructionScript`)