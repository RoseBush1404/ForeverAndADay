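; A spline-based wire actor for mechanisms that visually shows power switching on and off.
; The construction script tiles Z-forward spline mesh segments along the spline, sized by mesh length and actor X scale, with clamped tangents.
; At BeginPlay it binds to the MechanismActionComponent's activate and deactivate events and creates dynamic wire materials for each segment.
; Power events play or reverse a timeline that drives the materials' Blend parameter.
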(event `self.ReceiveBeginPlay`
  (add `/Game/Dynamic/Mechanisms/MechanismActionComponent.OnMechanismActionActivate` (`self.MechanismActionComponent`) (`|CreateDelegate` :!event `TurnPowerOn`))
  (add `/Game/Dynamic/Mechanisms/MechanismActionComponent.OnMechanismActionDeactivate` (`self.MechanismActionComponent`) (`|CreateDelegate` :!event `TurnPowerOff`))
  (for _array_element (`self.SplineMeshes`)
    (bind _returnvalue (`PrimitiveComponent.CreateDynamicMaterialInstance` _array_element 0 "/Game/Static/PuzzlePanel/Wires/M_Wire.M_Wire" "None"))
    (`KismetArrayLibrary.Array_AddUnique` (`self.WireMaterials`) _returnvalue)))

(event `TurnPowerOn`
  (bind (_direction _alpha) (`Timeline|WirePowerLerp` :!via `PlayFromStart` :!label _label)
    (:`Update`
      (`MaterialInstanceDynamic.SetScalarParameterValue` (`self.WireMaterials`) "Blend" _alpha))))

(event `TurnPowerOff`
  (goto _label :!via `ReverseFromEnd`))

(fn `UserConstructionScript`
  (bind _returnvalue_x (`KismetMathLibrary.BreakVector` (`self.GetActorScale3D`)))
  (bind _spline (`self.Spline`))
  (bind _spline_2 (`self.Spline`))
  (set `self.SectionLength` (* _returnvalue_x (`self.MeshLength`)))
  (for _index (range (+ (`KismetMathLibrary.FTrunc` (/ (`SplineComponent.GetSplineLength` (`self.Spline`)) (`self.SectionLength`))) 1))
    (bind _returnvalue (`AddComponent|NODE_AddSplineMeshComponent-0`))
    (`SplineMeshComponent.SetForwardAxis` _returnvalue "Z" true)
    (bind _returnvalue_2 (* _index (`self.SectionLength`)))
    (bind _returnvalue_3 (* (+ _index 1) (`self.SectionLength`)))
    (`SplineMeshComponent.SetStartAndEnd` _returnvalue (`SplineComponent.GetLocationAtDistanceAlongSpline` _spline_2 _returnvalue_2 "Local") (`KismetMathLibrary.ClampVectorSize` (`SplineComponent.GetTangentAtDistanceAlongSpline` _spline_2 _returnvalue_2 "Local") 0.0 (`self.SectionLength`)) (`SplineComponent.GetLocationAtDistanceAlongSpline` _spline _returnvalue_3 "Local") (`KismetMathLibrary.ClampVectorSize` (`SplineComponent.GetTangentAtDistanceAlongSpline` _spline _returnvalue_3 "Local") 0.0 (`self.SectionLength`)) true)
    (`KismetArrayLibrary.Array_AddUnique` (`self.SplineMeshes`) _returnvalue)))