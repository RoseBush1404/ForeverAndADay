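; Player controller Blueprint that routes player input to whichever pawn it currently possesses.
; Each action (Use, Exit, Sprint, Reset) forwards separate pressed and released messages, and each movement and look axis forwards its value.
; Calls go through interface-style messages on the controlled pawn, so the controller holds no gameplay logic and pawns decide how to respond.
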(event `InputAction|Pause`
  (params (Key :type "Key Structure")))

(event `InputAction|Use`
  (params (Key :type "Key Structure"))
  (bind _returnvalue (`self.K2_GetPawn`))
  (:`Pressed`
    (message `/Game/Dynamic/Character/I_InputControls.UsePressed` _returnvalue))
  (:`Released`
    (message `/Game/Dynamic/Character/I_InputControls.UseReleased` _returnvalue)))

(event `InputAxis|MoveForward/Backward`
  (params (AxisValue :type "Float (single-precision)"))
  (message `/Game/Dynamic/Character/I_InputControls.MoveForward/Backward` (`self.K2_GetPawn`) AxisValue))

(event `InputAxis|MoveRight/Left`
  (params (AxisValue :type "Float (single-precision)"))
  (message `/Game/Dynamic/Character/I_InputControls.MoveRight/Left` (`self.K2_GetPawn`) AxisValue))

(event `InputAxis|Turn`
  (params (AxisValue :type "Float (single-precision)"))
  (message `/Game/Dynamic/Character/I_InputControls.Turn` (`self.K2_GetPawn`) AxisValue))

(event `InputAxis|LookUp/Down`
  (params (AxisValue :type "Float (single-precision)"))
  (message `/Game/Dynamic/Character/I_InputControls.LookUp/Down` (`self.K2_GetPawn`) AxisValue))

(event `InputAction|Exit`
  (params (Key :type "Key Structure"))
  (bind _returnvalue (`self.K2_GetPawn`))
  (:`Pressed`
    (message `/Game/Dynamic/Character/I_InputControls.ExitPressed` _returnvalue))
  (:`Released`
    (message `/Game/Dynamic/Character/I_InputControls.ExitReleased` _returnvalue)))

(event `InputAction|Sprint`
  (params (Key :type "Key Structure"))
  (bind _returnvalue (`self.K2_GetPawn`))
  (:`Pressed`
    (message `/Game/Dynamic/Character/I_InputControls.SprintPressed` _returnvalue))
  (:`Released`
    (message `/Game/Dynamic/Character/I_InputControls.SprintReleased` _returnvalue)))

(event `InputAction|Reset`
  (params (Key :type "Key Structure"))
  (bind _returnvalue (`self.K2_GetPawn`))
  (:`Pressed`
    (message `/Game/Dynamic/Character/I_InputControls.ResetPressed` _returnvalue))
  (:`Released`
    (message `/Game/Dynamic/Character/I_InputControls.ResetReleased` _returnvalue)))

(fn `UserConstructionScript`)